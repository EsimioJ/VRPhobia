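; BP_Affresco is a fresco puzzle piece that can be picked up and dropped into its correct place.
; Construction uses the four- or sixteen-piece setting and Position to set material parameters selecting the piece's image tile.
; Pickup attaches it to a "foto" socket; Drop snaps it to CorrectLocation and CorrectRotation when close.
; It then counts placed pieces across all instances, driving a punch sound, material flash timeline and completion timelines.
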(event EventBeginPlay)

(event Collision|EventActorBeginOverlap
  (params (OtherActor :type Actor%20Object%20Reference)))

(event EventTick
  (params (DeltaSeconds :type Float%20%28single-precision%29)))

(event EventPickup
  (params (AttachTo :type Scene%20Component%20Object%20Reference))
  (Physics|SetSimulatePhysics (Variables|Default|GetStaticMesh) false)
  (Transformation|AttachComponentToComponent (VehicleSound|GetRootComponent) AttachTo "foto" "KeepWorld" "KeepWorld" "KeepWorld" false))

(event EventDrop
  (Physics|SetSimulatePhysics (Variables|Default|GetStaticMesh) false)
  (Transformation|DetachFromActor "KeepWorld" "KeepWorld" "KeepWorld")
  (if (Math|Vector|Equal(Vector) (Transformation|GetActorLocation) (Variables|Default|GetCorrectLocation) 1e+01)
    (Transformation|SetActorTransform (Math|Transform|MakeTransform (Variables|Default|GetCorrectLocation) (Variables|Default|GetCorrectRotation) (Transformation|GetActorScale3D)))
    (bind _outactors (Actor|GetAllActorsOfClass "BP_Affresco_C"))
    (for _array_element _outactors
      (if (Math|Vector|Equal(Vector) (Transformation|GetActorLocation _array_element) (Variables|BP_Affresco_C|GetCorrectLocation _array_element) 15.0)
        (bind _result (Math|Integer|IncrementInt (Variables|Default|GetSlotOk))
          (:%20%20
            (|CollapseGraph_0
              (:NewParam2
                (if (== _result (+ (Variables|Default|GetDivide) 2))
                  (bind _outactors_2 (Actor|GetAllActorsOfClass "BP_Affresco_C"))
                  (for _array_element_2 _outactors_2
                    (Components|Timeline|PlayfromStart (Variables|BP_Affresco_C|GetTimeline_0 _array_element_2))))))))
        (else
          (Variables|Default|SetSlotOk 0))))))

(fn ConstructionScript
  (switch Utilities|FlowControl|Switch|SwitchonEN_Affresco (Variables|Default|GetEN_Affresco)
    (:NewEnumerator0
      (Rendering|Material|SetScalarParameterValueonMaterials (Variables|Default|Getaffresco) "Divide" 4.0)
      (switch int (Variables|Default|GetPosition)
        (:0
          (Rendering|Material|SetScalarParameterValueonMaterials (Variables|Default|Getaffresco) "Horizontal" 0.0)
          (Rendering|Material|SetScalarParameterValueonMaterials (Variables|Default|Getaffresco) "Vertical" 0.0))
        (:1
          (Rendering|Material|SetScalarParameterValueonMaterials (Variables|Default|Getaffresco) "Horizontal" 1.0)
          (Rendering|Material|SetScalarParameterValueonMaterials (Variables|Default|Getaffresco) "Vertical" 0.0))
        (:2
          (Rendering|Material|SetScalarParameterValueonMaterials (Variables|Default|Getaffresco) "Horizontal" 0.0)
          (Rendering|Material|SetScalarParameterValueonMaterials (Variables|Default|Getaffresco) "Vertical" 1.0))
        (:3
          (Rendering|Material|SetScalarParameterValueonMaterials (Variables|Default|Getaffresco) "Horizontal" 1.0)
          (Rendering|Material|SetScalarParameterValueonMaterials (Variables|Default|Getaffresco) "Vertical" 1.0))))
    (:NewEnumerator1
      (Rendering|Material|SetScalarParameterValueonMaterials (Variables|Default|Getaffresco) "Divide" 8.0)
      (switch int (Variables|Default|GetPosition)
        (:0
          (CallFunction|Sets 0.0 0.0))
        (:1
          (CallFunction|Sets 1.0 0.0))
        (:2
          (CallFunction|Sets 2.0 0.0))
        (:3
          (CallFunction|Sets 3.0 0.0))
        (:4
          (CallFunction|Sets 0.0 1.0))
        (:5
          (CallFunction|Sets 1.0 1.0))
        (:6
          (CallFunction|Sets 2.0 1.0))
        (:7
          (CallFunction|Sets 3.0 1.0))
        (:8
          (CallFunction|Sets 0.0 2.0))
        (:9
          (CallFunction|Sets 1.0 2.0))
        (:10
          (CallFunction|Sets 2.0 2.0))
        (:11
          (CallFunction|Sets 3.0 2.0))
        (:12
          (CallFunction|Sets 0.0 3.0))
        (:13
          (CallFunction|Sets 1.0 3.0))
        (:14
          (CallFunction|Sets 2.0 3.0))
        (:15
          (CallFunction|Sets 3.0 3.0))))))

(fn Sets
  (params (Horizontal :type Float%20%28single-precision%29) (Vertical :type Float%20%28single-precision%29))
  (Rendering|Material|SetScalarParameterValueonMaterials (Variables|Default|Getaffresco) "Horizontal" Horizontal)
  (Rendering|Material|SetScalarParameterValueonMaterials (Variables|Default|Getaffresco) "Vertical" Vertical)
  (return))

(fn Flash)