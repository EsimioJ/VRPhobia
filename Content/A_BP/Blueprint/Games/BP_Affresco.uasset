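; Fresco puzzle piece that can be picked up, attached at the "foto" socket, and dropped to snap onto its correct transform when close enough.
; The construction script uses the piece count enum and Position to set material parameters that select its tile in a 2x2 or 4x4 grid.
; After a snap, it checks every piece's placement; a matching count triggers all pieces' timelines, a sound and a BP_BadgeCoin spawn.
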(event EventBeginPlay)

(event EventPickup
  (params (AttachTo :type Scene%20Component%20Object%20Reference) (Hand%20Skeletal%20Mesh :type Skeletal%20Mesh%20Component%20Object%20Reference) (MotionController :type Primitive%20Component%20Object%20Reference) (Actor :type Actor%20Object%20Reference))
  ;[1 1 1] Pickup
  (Physics|SetSimulatePhysics (Variables|Default|GetStaticMesh) false)
  (Transformation|AttachComponentToComponent (VehicleSound|GetRootComponent) AttachTo "foto" "KeepWorld" "KeepWorld" "KeepWorld" false))

(event EventDrop
  (params (Motion%20Controller :type Primitive%20Component%20Object%20Reference) (Hand%20Skeletal%20Mesh :type Skeletal%20Mesh%20Component%20Object%20Reference))
  (Physics|SetSimulatePhysics (Variables|Default|GetStaticMesh) false)
  (Transformation|DetachFromActor "KeepWorld" "KeepWorld" "KeepWorld")
  (if (Math|Vector|Equal(Vector) (Transformation|GetActorLocation) (Variables|Default|GetCorrectLocation) 1e+01)
    (Transformation|SetActorTransform (Math|Transform|MakeTransform (Variables|Default|GetCorrectLocation) (Variables|Default|GetCorrectRotation) (Transformation|GetActorScale3D)))
    (bind _outactors (Actor|GetAllActorsOfClass "BP_Affresco_C"))
    (for _array_element _outactors
      (if (Math|Vector|Equal(Vector) (Transformation|GetActorLocation _array_element) (Variables|BP_Affresco_C|GetCorrectLocation _array_element) 15.0)
        (bind _result (Math|Integer|IncrementInt (Variables|Default|GetSlotOk))
          (:%20%20
            (Variables|Default|SetSlotOk _result)
            (Components|Timeline|PlayfromStart (Variables|Default|GetTimeline_0))))
        (else
          (Variables|Default|SetSlotOk 0))))
    (if (== (Variables|Default|GetSlotOk) (* (Variables|Default|GetDivide) 2))
      (bind _outactors_2 (Actor|GetAllActorsOfClass "BP_Affresco_C"))
      (for _array_element_2 _outactors_2
        (Components|Timeline|PlayfromStart (Variables|BP_Affresco_C|GetTimeline_0 _array_element_2)))
      (Audio|PlaySound2D "/Game/StarterContent/Audio/Collapse01.Collapse01" 1.0 1.0 0.0 0 0)
      (Rendering|Material|SetScalarParameterValueonMaterials (Variables|Default|Getaffresco) "Flash" (Math|Interpolation|FInterpTo 0.0 1.0 (Utilities|Time|GetWorldDeltaSeconds) 2.0))
      (Game|SpawnActorfromClass "/Game/A_BP/Blueprint/BP_BadgeCoin.BP_BadgeCoin_C" (Transformation|GetWorldTransform (Variables|Default|GetScene)) "Undefined" 0 (Variables|Default|GetBadge%20Text) (Variables|Default|GetBadge%20Texture) 0)
      (else
        (|CollapseGraph_0_2
          (:NewParam2
            (Variables|Default|SetSlotOk 0)))))))

(fn ConstructionScript
  (switch Utilities|FlowControl|Switch|SwitchonEN_Affresco (Variables|Default|GetEN_Affresco)
    (:NewEnumerator0
      (Rendering|Material|SetScalarParameterValueonMaterials (Variables|Default|Getaffresco) "Divide" 2.0)
      (switch int (Variables|Default|GetPosition)
        (:0
          (Rendering|Material|SetScalarParameterValueonMaterials (Variables|Default|Getaffresco) "Horizontal" 0.0)
          (Rendering|Material|SetScalarParameterValueonMaterials (Variables|Default|Getaffresco) "Vertical" 0.0))
        (:1
          (Rendering|Material|SetScalarParameterValueonMaterials (Variables|Default|Getaffresco) "Horizontal" 1.0)
          (Rendering|Material|SetScalarParameterValueonMaterials (Variables|Default|Getaffresco) "Vertical" 0.0))
        (:2
          (Rendering|Material|SetScalarParameterValueonMaterials (Variables|Default|Getaffresco) "Horizontal" 0.0)
          (Rendering|Material|SetScalarParameterValueonMaterials (Variables|Default|Getaffresco) "Vertical" 1.0))
        (:3
          (Rendering|Material|SetScalarParameterValueonMaterials (Variables|Default|Getaffresco) "Horizontal" 1.0)
          (Rendering|Material|SetScalarParameterValueonMaterials (Variables|Default|Getaffresco) "Vertical" 1.0))))
    (:NewEnumerator1
      (Rendering|Material|SetScalarParameterValueonMaterials (Variables|Default|Getaffresco) "Divide" 4.0)
      (switch int (Variables|Default|GetPosition)
        (:0
          (CallFunction|Sets 0.0 0.0))
        (:1
          (CallFunction|Sets 1.0 0.0))
        (:2
          (CallFunction|Sets 2.0 0.0))
        (:3
          (CallFunction|Sets 3.0 0.0))
        (:4
          (CallFunction|Sets 0.0 1.0))
        (:5
          (CallFunction|Sets 1.0 1.0))
        (:6
          (CallFunction|Sets 2.0 1.0))
        (:7
          (CallFunction|Sets 3.0 1.0))
        (:8
          (CallFunction|Sets 0.0 2.0))
        (:9
          (CallFunction|Sets 1.0 2.0))
        (:10
          (CallFunction|Sets 2.0 2.0))
        (:11
          (CallFunction|Sets 3.0 2.0))
        (:12
          (CallFunction|Sets 0.0 3.0))
        (:13
          (CallFunction|Sets 1.0 3.0))
        (:14
          (CallFunction|Sets 2.0 3.0))
        (:15
          (CallFunction|Sets 3.0 3.0))))))

(fn Sets
  (params (Horizontal :type Float%20%28single-precision%29) (Vertical :type Float%20%28single-precision%29))
  (Rendering|Material|SetScalarParameterValueonMaterials (Variables|Default|Getaffresco) "Horizontal" Horizontal)
  (Rendering|Material|SetScalarParameterValueonMaterials (Variables|Default|Getaffresco) "Vertical" Vertical)
  (return))

(fn Flash)