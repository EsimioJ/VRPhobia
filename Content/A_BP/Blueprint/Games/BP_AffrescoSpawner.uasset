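; VR push-button actor that cycles the texture shown on every BP_Affresco in the level.
; Overlap with a BP_MotionController starts tracking; Tick projects hand movement onto the button's up axis, moving it up to a travel limit.
; A full press calls ChangeImage, which applies the next array texture through dynamic material instances, then starts the button's return.
; A separate sphere overlap rumbles the right controller and switches its hand grip animation.
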(event OnComponentBeginOverlap(Sphere)
  (params (OverlappedComponent :type Primitive%20Component%20Object%20Reference) (OtherActor :type Actor%20Object%20Reference) (OtherComp :type Primitive%20Component%20Object%20Reference) (OtherBodyIndex :type Integer) (bFromSweep :type Boolean) (SweepResult :type Hit%20Result%20Structure%20%28by%20ref%29))
  (Development|PrintString "Hello")
  (bind _asmotion_controller_pawn (Utilities|Casting|CastToMotionControllerPawn OtherActor))
  (Default|RumbleController (Variables|/Game/VirtualRealityBP/Blueprints/MotionControllerPawn.MotionControllerPawn_C|GetRightController _asmotion_controller_pawn) 1.0)
  (bind _asright_hand_anim_bp (Utilities|Casting|CastToRightHand_AnimBP (Components|SkeletalMesh|GetAnimInstance (Variables|/Game/VirtualRealityBP/Blueprints/BP_MotionController.BP_MotionController_C|GetHandMesh (Variables|/Game/VirtualRealityBP/Blueprints/MotionControllerPawn.MotionControllerPawn_C|GetRightController _asmotion_controller_pawn)))))
  (Variables|/Game/VirtualReality/Mannequin/Animations/RightHand_AnimBP.RightHand_AnimBP_C|SetChangeAnimation _asright_hand_anim_bp true)
  (Variables|/Game/VirtualReality/Mannequin/Animations/RightHand_AnimBP.RightHand_AnimBP_C|SetGripState _asright_hand_anim_bp "NewEnumerator3"))

(event OnComponentBeginOverlap(ButtonA)
  (params (OverlappedComponent :type Primitive%20Component%20Object%20Reference) (OtherActor :type Actor%20Object%20Reference) (OtherComp :type Primitive%20Component%20Object%20Reference) (OtherBodyIndex :type Integer) (bFromSweep :type Boolean) (SweepResult :type Hit%20Result%20Structure%20%28by%20ref%29))
  (bind _asbp_motion_controller (Utilities|Casting|CastToBP_MotionController OtherActor))
  (Variables|Default|SetMotion%20Controller (Variables|/Game/VirtualRealityBP/Blueprints/BP_MotionController.BP_MotionController_C|GetMotionController _asbp_motion_controller))
  (Variables|Default|SetButtonComponent (Variables|Default|GetButtonA))
  (Variables|Default|SetbIsTrackingA true)
  (Variables|Default|SetMC%20Initial%20Location (Transformation|GetWorldLocation (Variables|Default|GetMotion%20Controller))))

(event OnComponentEndOverlap(Sphere)
  (params (OverlappedComponent :type Primitive%20Component%20Object%20Reference) (OtherActor :type Actor%20Object%20Reference) (OtherComp :type Primitive%20Component%20Object%20Reference) (OtherBodyIndex :type Integer))
  (bind _asmotion_controller_pawn (Utilities|Casting|CastToMotionControllerPawn (Variables|Default|GetMotion%20Controller)))
  (bind _asright_hand_anim_bp (Utilities|Casting|CastToRightHand_AnimBP (Components|SkeletalMesh|GetAnimInstance (Variables|/Game/VirtualRealityBP/Blueprints/BP_MotionController.BP_MotionController_C|GetHandMesh (Variables|/Game/VirtualRealityBP/Blueprints/MotionControllerPawn.MotionControllerPawn_C|GetRightController _asmotion_controller_pawn)))))
  (Variables|/Game/VirtualReality/Mannequin/Animations/RightHand_AnimBP.RightHand_AnimBP_C|SetChangeAnimation _asright_hand_anim_bp false)
  (Variables|/Game/VirtualReality/Mannequin/Animations/RightHand_AnimBP.RightHand_AnimBP_C|SetGripState _asright_hand_anim_bp "NewEnumerator0"))

(event Custom|ChangeImage
  (if (== (Variables|Default|GetSlotTexture) (- (Utilities|Array|Length (Variables|Default|GetValue)) 1))
    (Variables|Default|SetSlotTexture 0)
    (else
      (CallFunction|ChangeTexture))))

(event EventBeginPlay
  (Variables|Default|SetButtonA%20Initial%20Location (Transformation|GetWorldLocation (Variables|Default|GetButtonA))))

(event EventTick
  (params (DeltaSeconds :type Float%20%28single-precision%29))
  (if (Variables|Default|GetbIsTrackingA)
    (bind _output_get (CallFunction|ButtonsMovement (Variables|Default|GetButtonComponent)))
    (if _output_get
      (CallFunction|ChangeImage))
    (elif (Variables|Default|GetButtonA%20IsReturning)
      (CallFunction|ButtonReturn (Variables|Default|GetButtonComponent)))))

(fn ConstructionScript)

(fn ChangeTexture
  (bind _outactors (Actor|GetAllActorsOfClass "/Game/A_BP/Blueprint/Games/BP_Affresco.BP_Affresco_C"))
  (for _array_element _outactors
    (bind _returnvalue (Rendering|Material|CreateDynamicMaterialInstance (Variables|/Game/A_BP/Blueprint/Games/BP_Affresco.BP_Affresco_C|Getaffresco _array_element) 0 (Rendering|Material|GetMaterial (Variables|/Game/A_BP/Blueprint/Games/BP_Affresco.BP_Affresco_C|Getaffresco _array_element) 0) "None" :!class /Script/Engine.PrimitiveComponent))
    (Rendering|Material|SetTextureParameterValue _returnvalue "Texture" (Utilities|Array|Get(acopy) (Variables|Default|GetValue) (Variables|Default|GetSlotTexture))))
  (Variables|Default|SetSlotTexture (+ (Variables|Default|GetSlotTexture) 1))
  (return))

(fn ButtonsMovement
  (params (Button :type Scene%20Component%20Object%20Reference))
  (Variables|Default|SetButtonA%20Current%20Travel (Math|Float|Clamp(Float) (Math|Float|Absolute(Float) (Math|Vector|VectorLength (Math|Vector|ProjectVectorontoVector (- (Transformation|GetWorldLocation (Variables|Default|GetMotion%20Controller)) (Variables|Default|GetMC%20Initial%20Location)) (Math|Vector|GetUpVector Button)))) 0.0 (Variables|Default|GetButtonA%20Max%20Travel)))
  (bind _output_get (Variables|Default|SetButtonA%20Current%20Location (- (Variables|Default|GetButtonA%20Initial%20Location) (* (Math|Vector|GetUpVector Button) (Variables|Default|GetButtonA%20Current%20Travel)))))
  (Transformation|SetWorldLocation Button _output_get false false)
  (if (>= (Variables|Default|GetButtonA%20Current%20Travel) (Variables|Default|GetButtonA%20Max%20Travel))
    (Variables|Default|SetbIsTrackingA false)
    (Variables|Default|SetButtonA%20IsReturning true)
    (return true)
    (else
      (return false))))

(fn ButtonReturn
  (params (Button :type Scene%20Component%20Object%20Reference))
  (bind _output_get (Variables|Default|SetButtonA%20Current%20Location (Math|Interpolation|VInterpTo (Variables|Default|GetButtonA%20Initial%20Location) (Variables|Default|GetButtonA%20Current%20Location) (Utilities|Time|GetWorldDeltaSeconds) 2.0)))
  (Transformation|SetWorldLocation Button _output_get false false)
  (if (Class|KismetMathLibrary|EqualExactlyVectorVector (Variables|Default|GetButtonA%20Initial%20Location) (Variables|Default|GetButtonA%20Current%20Location))
    (Variables|Default|SetButtonA%20IsReturning false)
    (return)
    (else
      (return))))