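; Wall sign for a picture placement mini-game that awards a badge coin when the puzzle is solved.
; Its isGameFinished event counts Bp_picture actors flagged CorrectLocation, zeroing the count and stopping at the first misplaced one.
; A count of four spawns a BP_BadgeCoin at the Scene component's transform with the sign's badge text and texture.
; BeginPlay holds only a delay, and the graph's own call to the check is unconnected.
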(event Custom|isGameFinished
  (bind _outactors (Actor|GetAllActorsOfClass "/Game/A_BP/Blueprint/Games/bp_picture.bp_picture_C"))
  (bind _array_element (Utilities|Array|ForEachLoopwithBreak _outactors :!label _label)
    (:LoopBody
      (if (Variables|/Game/A_BP/Blueprint/Games/bp_picture.bp_picture_C|GetCorrectLocation _array_element)
        (bind _result (Math|Integer|IncrementInt (Variables|Default|GetTotalCorrect))
          (:%20%20
            (Variables|Default|SetTotalCorrect _result)))
        (else
          (Variables|Default|SetTotalCorrect 0)
          (goto _label Break))))
    (:Completed
      (if (== (Variables|Default|GetTotalCorrect) 4)
        (Game|SpawnActorfromClass "/Game/A_BP/Blueprint/BP_BadgeCoin.BP_BadgeCoin_C" (Transformation|GetWorldTransform (Variables|Default|GetScene)) "Undefined" 0 (Variables|Default|GetBadge%20Text) (Variables|Default|GetBadge%20Texture) 0)))))

(event EventBeginPlay
  (Utilities|FlowControl|Delay 2.0))

(fn ConstructionScript)