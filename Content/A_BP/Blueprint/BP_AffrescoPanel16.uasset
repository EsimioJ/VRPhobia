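; Fresco puzzle panel that spawns BP_Affresco pieces on its cube slots and scrambles their positions.
; On BeginPlay it enables input, waits, then spawns a piece at each of up to four cubes, passing slot index, grid division and correct transform.
; After another delay it shuffles the recorded slot locations and teleports every BP_Affresco in the level onto them.
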(event EventBeginPlay
  (bind _newvar_1 (Variables|Default|GetNewVar_1))
  (bind _output (Utilities|Array|Get(acopy) _newvar_1))
  (Input|EnableInput (Game|GetPlayerController 0))
  (Utilities|FlowControl|Delay 5.0)
  (for _index (range 0 (Variables|Default|Getnumberslots))
    (switch int _index
      (:0
        (CallFunction|SpawnAffresco _index (Variables|Default|GetCube)))
      (:1
        (CallFunction|SpawnAffresco _index (Variables|Default|GetCube1)))
      (:2
        (CallFunction|SpawnAffresco _index (Variables|Default|GetCube2)))
      (:3
        (CallFunction|SpawnAffresco _index (Variables|Default|GetCube3)))))
  (Utilities|FlowControl|Delay 1.5)
  (Utilities|Array|Shuffle (Variables|Default|GetNewVar_1))
  (Utilities|Array|Shuffle (Variables|Default|GetNewVar_1))
  (bind _outactors (Actor|GetAllActorsOfClass "/Game/A_BP/Blueprint/BP_Affresco.BP_Affresco_C"))
  (for _array_element _outactors
    (Transformation|SetActorLocation _array_element _output false true)
    (Utilities|Array|RemoveItem (Variables|Default|GetNewVar_1) _output)))

(event Collision|EventActorBeginOverlap
  (params (OtherActor :type Actor%20Object%20Reference)))

(event EventTick
  (params (DeltaSeconds :type Float%20%28single-precision%29)))

(fn ConstructionScript)

(fn SpawnAffresco
  (params (Position :type Integer) (Target :type Scene%20Component%20Object%20Reference))
  (bind _returnvalue (Transformation|GetWorldLocation Target))
  (Game|SpawnActorfromClass "/Game/A_BP/Blueprint/BP_Affresco.BP_Affresco_C" (Transformation|GetWorldTransform Target) "Undefined" 0 Position 2 _returnvalue (Transformation|GetWorldRotation Target) 0)
  (Utilities|Array|Add (Variables|Default|GetNewVar_1) _returnvalue)
  (return))