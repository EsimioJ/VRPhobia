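; BP_BadgeCoin is a collectible badge coin that can be picked up and added to the player's badge inventory.
; On BeginPlay one timeline spins and slides the cylinder mesh, then a second drives a small vertical float.
; Pickup stops both timelines, attaches to a "foto" socket and passes its text and texture through GM_VrPhobia into the badge menu's OnidiofobiaGrid.
; Drop detaches and destroys the coin.
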(event EventBeginPlay
  (bind _cylinder (Variables|Default|GetCylinder))
  (bind _cylinder_2 (Variables|Default|GetCylinder))
  (bind _relativerotation (Variables|/Script/Engine.SceneComponent|GetRelativeRotation _cylinder))
  (bind _relativelocation (Variables|/Script/Engine.SceneComponent|GetRelativeLocation _cylinder))
  (bind _relativelocation_2 (Variables|/Script/Engine.SceneComponent|GetRelativeLocation _cylinder_2))
  (bind _newtrack_0 (Timeline|Timeline_0 Play)
    (:Update
      (Transformation|SetRelativeRotation _cylinder (Math|Rotator|MakeRotator (.roll _relativerotation) (.pitch _relativerotation) (Math|Float|MapRangeClamped _newtrack_0 0.0 1.0 0.0 1.08e+03)) false false)
      (Transformation|SetRelativeLocation _cylinder (Math|Vector|MakeVector (.x _relativelocation) (Math|Float|MapRangeClamped _newtrack_0 0.0 1.0 0.0 3e+01) (.z _relativelocation)) false false))
    (:Finished
      (bind _newtrack_0_2 (Timeline|Timeline_1 Play)
        (:Update
          (Transformation|SetRelativeLocation _cylinder_2 (Math|Vector|MakeVector (.x _relativelocation_2) (.y _relativelocation_2) (Math|Float|MapRangeClamped _newtrack_0_2 -1.0 1.0 -2.0 2.0)) false false))))))

(event Collision|EventActorBeginOverlap
  (params (OtherActor :type Actor%20Object%20Reference)))

(event EventTick
  (params (DeltaSeconds :type Float%20%28single-precision%29)))

(event EventPickup
  (params (AttachTo :type Scene%20Component%20Object%20Reference) (Skeletal%20Mesh :type Skeletal%20Mesh%20Component%20Object%20Reference) (MotionController :type Primitive%20Component%20Object%20Reference))
  (Audio|Components|Audio|Stop (Variables|Default|GetTimeline_1))
  (Transformation|AttachComponentToComponent (VehicleSound|GetRootComponent) AttachTo "foto" "KeepWorld" "KeepWorld" "KeepWorld" false)
  (bind _returnvalue (Actor|GetActorOfClass "/Game/A_BP/Blueprint/BP_GameMenu.BP_GameMenu_C"))
  (bind _asw_badge_menu (Utilities|Casting|CastTow_BadgeMenu (UserInterface|GetWidget (Variables|/Game/A_BP/Blueprint/BP_GameMenu.BP_GameMenu_C|GetWidget _returnvalue))))
  (bind _asgm_vr_phobia (Utilities|Casting|CastToGM_VrPhobia (Game|GetGameMode)))
  (Default|BadgeInventoryAdd _asgm_vr_phobia (Variables|Default|GetBadgeText) (Variables|Default|GetBadgeTexture) (Variables|/Game/A_BP/Widget/w_BadgeMenu.w_BadgeMenu_C|GetOnidiofobiaGrid _asw_badge_menu)))

(event EventDrop
  (Transformation|DetachFromActor "KeepWorld" "KeepWorld" "KeepWorld")
  (Actor|DestroyActor))

(fn ConstructionScript)