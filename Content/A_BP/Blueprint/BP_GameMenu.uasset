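; BP_GameMenu is an unfinished game menu actor with a Cube component and a distance check against the VR player's camera.
; Each Tick casts player controller 0, rather than its pawn, to MotionControllerPawn and compares camera-to-Cube distance with a fixed threshold.
; The branch leads to no action, and the node that hides DefaultSceneRoot is unconnected, so the menu's visibility never changes.
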(event EventBeginPlay)

(event Collision|EventActorBeginOverlap
  (params (OtherActor :type Actor%20Object%20Reference)))

(event EventTick
  (params (DeltaSeconds :type Float%20%28single-precision%29))
  (bind _asmotion_controller_pawn (Utilities|Casting|CastToMotionControllerPawn (Game|GetPlayerController 0)))
  (if (>= (Math|Vector|Distance(Vector) (Transformation|GetWorldLocation (Variables|/Game/VirtualRealityBP/Blueprints/MotionControllerPawn.MotionControllerPawn_C|GetCamera _asmotion_controller_pawn)) (Transformation|GetWorldLocation (Variables|Default|GetCube))) 2e+02)
    _))

(fn ConstructionScript)