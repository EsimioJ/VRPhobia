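; Fresco puzzle panel with 16 slots that spawns BP_Affresco pieces and scrambles their positions.
; The construction script lays out the slot components in four evenly spaced rows.
; After a delay on BeginPlay, it spawns a piece per slot, passing its index and correct transform, and records the location.
; It then shuffles those locations and teleports every BP_Affresco in the level onto them.
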(event EventBeginPlay
  (bind _newvar_1 (Variables|Default|GetNewVar_1))
  (bind _output (Utilities|Array|Get(acopy) _newvar_1))
  (Utilities|FlowControl|Delay 2.0)
  (for _index (range 0 (Variables|Default|Getnumberslots))
    (switch int _index
      (:0
        (CallFunction|SpawnAffresco _index (Variables|Default|GetCube)))
      (:1
        (CallFunction|SpawnAffresco _index (Variables|Default|GetCube1)))
      (:2
        (CallFunction|SpawnAffresco _index (Variables|Default|GetCube2)))
      (:3
        (CallFunction|SpawnAffresco _index (Variables|Default|GetCube3)))
      (:4
        (CallFunction|SpawnAffresco _index (Variables|Default|GetCube4)))
      (:5
        (CallFunction|SpawnAffresco _index (Variables|Default|GetCube5)))
      (:6
        (CallFunction|SpawnAffresco _index (Variables|Default|GetCube6)))
      (:7
        (CallFunction|SpawnAffresco _index (Variables|Default|GetCube7)))
      (:8
        (goto _label execute4))
      (:9
        (goto _label execute3))
      (:10
        (|CollapseGraph_1 _index :!label _label))
      (:11
        (goto _label execute2))
      (:12
        (goto _label_2 execute4))
      (:13
        (goto _label_2 execute3))
      (:14
        (|CollapseGraph_2 _index _index _index _index :!label _label_2))
      (:15
        (goto _label_2 execute2))))
  (Utilities|FlowControl|Delay 1.5)
  (Utilities|Array|Shuffle (Variables|Default|GetNewVar_1))
  (Utilities|Array|Shuffle (Variables|Default|GetNewVar_1))
  (bind _outactors (Actor|GetAllActorsOfClass "/Game/A_BP/Blueprint/BP_Affresco.BP_Affresco_C"))
  (for _array_element _outactors
    (Transformation|SetActorLocation _array_element _output false true)
    (Utilities|Array|RemoveItem (Variables|Default|GetNewVar_1) _output)))

(event Collision|EventActorBeginOverlap
  (params (OtherActor :type Actor%20Object%20Reference)))

(event EventTick
  (params (DeltaSeconds :type Float%20%28single-precision%29)))

(fn ConstructionScript
  (for _array_element (Components|GetChildrenComponents (Variables|Default|Get1Row5) false)
    (Transformation|SetRelativeLocation _array_element (Math|Vector|MakeVector (+ (Variables|Default|Getlocation) (Variables|Default|Getdistance)) 0.0 0.0) false false)
    (Variables|Default|Setlocation (+ (Variables|Default|Getlocation) (Variables|Default|Getdistance))))
  (Variables|Default|Setlocation 0.0)
  (for _array_element_2 (Components|GetChildrenComponents (Variables|Default|Get1Row4) false)
    (Transformation|SetRelativeLocation _array_element_2 (Math|Vector|MakeVector (+ (Variables|Default|Getlocation) (Variables|Default|Getdistance)) 0.0 25.0) false false)
    (Variables|Default|Setlocation (+ (Variables|Default|Getlocation) (Variables|Default|Getdistance))))
  (Variables|Default|Setlocation 0.0)
  (for _array_element_3 (Components|GetChildrenComponents (Variables|Default|Get1Row3) false)
    (Transformation|SetRelativeLocation _array_element_3 (Math|Vector|MakeVector (+ (Variables|Default|Getlocation) (Variables|Default|Getdistance)) 0.0 5e+01) false false)
    (Variables|Default|Setlocation (+ (Variables|Default|Getlocation) (Variables|Default|Getdistance))))
  (Variables|Default|Setlocation 0.0)
  (for _array_element_4 (Components|GetChildrenComponents (Variables|Default|Get1Row) false)
    (Transformation|SetRelativeLocation _array_element_4 (Math|Vector|MakeVector (+ (Variables|Default|Getlocation) (Variables|Default|Getdistance)) 0.0 75.0) false false)
    (Variables|Default|Setlocation (+ (Variables|Default|Getlocation) (Variables|Default|Getdistance)))))

(fn SpawnAffresco
  (params (Position :type Integer) (Target :type Scene%20Component%20Object%20Reference))
  (bind _returnvalue (Transformation|GetWorldLocation Target))
  (Game|SpawnActorfromClass "/Game/A_BP/Blueprint/BP_Affresco.BP_Affresco_C" (Transformation|GetWorldTransform Target) "Undefined" 0 Position (Variables|Default|GetDivide) _returnvalue (Transformation|GetWorldRotation Target) (Variables|Default|GetEN%20Affresco) 0)
  (Utilities|Array|Add (Variables|Default|GetNewVar_1) _returnvalue)
  (return))