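; VR door Blueprint that the player grabs with a motion controller and swings by moving their hand.
; Pickup finds an overlapping BP_MotionController in the Box and marks the door grabbed.
; While grabbed, Tick calls RotatingDoor, which yaws the Scene component by a look-at between hand and actor, clamped to min and max limits.
; Drop, or the controller leaving the Box, releases it.
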(event OnComponentBeginOverlap(Box)
  (params (OverlappedComponent :type Primitive%20Component%20Object%20Reference) (OtherActor :type Actor%20Object%20Reference) (OtherComp :type Primitive%20Component%20Object%20Reference) (OtherBodyIndex :type Integer) (bFromSweep :type Boolean) (SweepResult :type Hit%20Result%20Structure%20%28by%20ref%29)))

(event OnComponentEndOverlap(Box)
  (params (OverlappedComponent :type Primitive%20Component%20Object%20Reference) (OtherActor :type Actor%20Object%20Reference) (OtherComp :type Primitive%20Component%20Object%20Reference) (OtherBodyIndex :type Integer))
  (bind _asbp_motion_controller (Utilities|Casting|CastToBP_MotionController OtherActor))
  (Variables|Default|SetbIsGrabbed false)
  (Variables|Default|SetAs%20BP%20Motion%20Controller _asbp_motion_controller)
  (Physics|SetSimulatePhysics (Variables|Default|GetDoor) false)
  (Transformation|DetachFromActor "KeepRelative" "KeepRelative" "KeepRelative"))

(event EventBeginPlay)

(event Collision|EventActorBeginOverlap
  (params (OtherActor :type Actor%20Object%20Reference)))

(event EventTick
  (params (DeltaSeconds :type Float%20%28single-precision%29))
  (if (Variables|Default|GetbIsGrabbed)
    (Utilities|IsValid (Variables|Default|GetAs%20BP%20Motion%20Controller)
      (:Is%20Valid
        (CallFunction|RotatingDoor (Transformation|GetWorldLocation (Variables|/Game/VirtualRealityBP/Blueprints/BP_MotionController.BP_MotionController_C|GetHandMesh (Variables|Default|GetAs%20BP%20Motion%20Controller)))))
      (:Is%20Not%20Valid
        (Variables|Default|SetbIsGrabbed false)))))

(event EventPickup
  (params (AttachTo :type Scene%20Component%20Object%20Reference))
  (bind _box (Variables|Default|GetBox))
  (bind _returnvalue (Transformation|GetWorldLocation _box))
  (Physics|SetSimulatePhysics (Variables|Default|GetDoor) false)
  (Transformation|AttachComponentToComponent (Variables|Default|GetScene1) AttachTo "foto" "KeepRelative" "KeepRelative" "KeepRelative" false)
  (bind _array_element (Utilities|Array|ForEachLoopwithBreak (Collision|GetOverlappingActors (Variables|Default|GetBox) 0 :!class /Script/Engine.PrimitiveComponent) :!label _label)
    (:LoopBody
      (bind _asbp_motion_controller (Utilities|Casting|CastToBP_MotionController _array_element))
      (Variables|Default|SetAs%20BP%20Motion%20Controller _asbp_motion_controller)
      (Variables|Default|SetbIsGrabbed true)
      (goto _label Break))
    (:Completed
      (if (Variables|Default|GetbIsGrabbed)
        (Utilities|IsValid (Variables|Default|GetAs%20BP%20Motion%20Controller)
          (:Is%20Valid
            (Variables|Default|SetInitial%20Location _returnvalue)
            (Variables|Default|SetDistance (Math|Vector|VectorLength (- (Transformation|GetWorldLocation (Variables|/Game/VirtualRealityBP/Blueprints/BP_MotionController.BP_MotionController_C|GetHandMesh (Variables|Default|GetAs%20BP%20Motion%20Controller))) _returnvalue)))))))))

(event EventDrop
  (Variables|Default|SetbIsGrabbed false)
  (Variables|Default|SetAs%20BP%20Motion%20Controller (stale OnComponentEndOverlap(Box) _asbp_motion_controller))
  (Physics|SetSimulatePhysics (Variables|Default|GetDoor) false)
  (Transformation|DetachFromActor "KeepRelative" "KeepRelative" "KeepRelative"))

(fn ConstructionScript
  (Transformation|AttachComponentToComponent (Variables|Default|GetCube) (Variables|Default|GetDoor) "None" "KeepRelative" "KeepRelative" "KeepRelative" true))

(fn RotatingDoor
  (params (NewParam :type Vector))
  (bind _returnvalue (Transformation|GetActorRotation))
  (Transformation|SetWorldRotation (Variables|Default|GetScene) (Math|Rotator|MakeRotator (.roll _returnvalue) (.pitch _returnvalue) (Math|Float|Clamp(Float) (.yaw (Math|Rotator|FindLookatRotation NewParam (Transformation|GetActorLocation))) (Variables|Default|GetMinRotation) (Variables|Default|GetMaxRotation))) false false))