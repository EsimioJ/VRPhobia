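; A numbered picture frame that can be picked up, dropped and snapped into its matching frame slot.
; The construction script uses Number to choose a snake texture for the picture's dynamic material.
; Pickup disables physics and attaches the actor to the given component.
; Drop finds the Bp_framesnap with the same number, then detaches and snaps to it if very close, otherwise re-enables physics.
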(event EventPickup
  (params (AttachTo :type Scene%20Component%20Object%20Reference))
  (Physics|SetSimulatePhysics (Variables|Default|GetFrame) false)
  (bind _returnvalue (Transformation|AttachComponentToComponent (VehicleSound|GetRootComponent) AttachTo "foto" "KeepWorld" "KeepWorld" "KeepWorld" false))
  (Development|PrintString (Utilities|String|ToString(Boolean) _returnvalue)))

(event EventDrop
  (bind _outactors (Actor|GetAllActorsOfClass "/Game/A_BP/Blueprint/bp_framesnap.bp_framesnap_C"))
  (bind _array_element (Utilities|Array|ForEachLoopwithBreak _outactors :!label _label)
    (:LoopBody
      (if (== (Variables|/Game/A_BP/Blueprint/bp_framesnap.bp_framesnap_C|Getpicture _array_element) (Variables|Default|GetNumber))
        (Variables|Default|SetArray%20Element _array_element)
        (goto _label Break)
        (else
          (Physics|SetSimulatePhysics (Variables|Default|GetFrame) true))))
    (:Completed
      (if (<= (Math|Vector|Distance(Vector) (Transformation|GetActorLocation (Variables|Default|GetArray%20Element)) (Transformation|GetActorLocation)) 1e+01)
        (Transformation|DetachFromActor "KeepWorld" "KeepWorld" "KeepWorld")
        (Physics|SetSimulatePhysics (Variables|Default|GetFrame) false)
        (Transformation|SetActorTransform (Math|Transform|MakeTransform (.location (Transformation|GetActorTransform (Variables|Default|GetArray%20Element))) (.rotation (Transformation|GetActorTransform (Variables|Default|GetArray%20Element))) (.scale (Transformation|GetActorTransform))) false true)
        (else
          (Physics|SetSimulatePhysics (Variables|Default|GetFrame) true))))))

(fn ConstructionScript
  (bind _returnvalue (Rendering|Material|CreateDynamicMaterialInstance (Rendering|Material|GetMaterial (Variables|Default|GetPicture) 0) "foto" "None" :!class /Script/Engine.KismetMaterialLibrary))
  (Variables|Default|SetDyn_Material_instance _returnvalue)
  (switch int (Variables|Default|GetNumber)
    (:0
      (Rendering|Material|SetTextureParameterValue (Variables|Default|GetDyn_Material_instance) "foto" "/Game/A_BP/Materials/Images/snakec1.snakec1")
      (Rendering|Material|SetMaterial (Variables|Default|GetPicture) 0 (Variables|Default|GetDyn_Material_instance)))
    (:1
      (Rendering|Material|SetTextureParameterValue (Variables|Default|GetDyn_Material_instance) "foto" "/Game/A_BP/Materials/Images/snakec1.snakec1")
      (Rendering|Material|SetMaterial (Variables|Default|GetPicture) 0 (Variables|Default|GetDyn_Material_instance)))
    (:2
      (Rendering|Material|SetTextureParameterValue (Variables|Default|GetDyn_Material_instance) "foto" "/Game/A_BP/Materials/Images/snakec2.snakec2")
      (Rendering|Material|SetMaterial (Variables|Default|GetPicture) 0 (Variables|Default|GetDyn_Material_instance)))
    (:3
      (Rendering|Material|SetTextureParameterValue (Variables|Default|GetDyn_Material_instance) "foto" "/Game/A_BP/Materials/Images/snakec3.snakec3")
      (Rendering|Material|SetMaterial (Variables|Default|GetPicture) 0 (Variables|Default|GetDyn_Material_instance)))
    (:4
      (Rendering|Material|SetTextureParameterValue (Variables|Default|GetDyn_Material_instance) "foto" "/Game/A_BP/Materials/Images/snakec4.snakec4")
      (Rendering|Material|SetMaterial (Variables|Default|GetPicture) 0 (Variables|Default|GetDyn_Material_instance)))))