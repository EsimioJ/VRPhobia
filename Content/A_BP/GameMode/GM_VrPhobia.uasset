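; GM_VrPhobia is the VR phobia game mode, providing helpers for awarding badges.
; BadgeInventoryAdd skips names already in BadgeInventory, otherwise records the name, adds a W_BadgeSlot to the given uniform grid (four in the first row, the rest in the second) and plays a click sound.
; BadgeOnScreen separately shows a fade-in W_BadgeObtained popup.
; BeginPlay is empty, and the event graph's badge test chains are disconnected.
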(event EventBeginPlay)

(fn ConstructionScript)

(fn BadgeonScreen
  (params (Icon%20Text :type Text) (Texture :type Texture%202D%20Object%20Reference))
  (bind _returnvalue (UserInterface|CreateWidget "/Game/A_BP/Widget/W_BadgeObtained.W_BadgeObtained_C" (Game|GetPlayerController 0)))
  (Variables|/Game/A_BP/Widget/W_BadgeSlot.W_BadgeSlot_C|SetIcon%20Text (Variables|/Game/A_BP/Widget/W_BadgeObtained.W_BadgeObtained_C|GetW_BadgeSlot _returnvalue) Icon%20Text)
  (Variables|/Game/A_BP/Widget/W_BadgeSlot.W_BadgeSlot_C|SetTexture (Variables|/Game/A_BP/Widget/W_BadgeObtained.W_BadgeObtained_C|GetW_BadgeSlot _returnvalue) Texture)
  (UserInterface|Viewport|AddtoViewport _returnvalue 0)
  (UserInterface|Animation|PlayAnimation _returnvalue (Variables|/Game/A_BP/Widget/W_BadgeObtained.W_BadgeObtained_C|Getfadein _returnvalue) 0.0 1 "Forward" 1.0 false)
  (return))

(fn BadgeInventoryAdd
  (params (Icon%20Text :type Text) (Texture :type Texture%202D%20Object%20Reference) (Target :type Uniform%20Grid%20Panel%20Object%20Reference))
  (bind _output_get (Variables|Default|SetIcon%20Text Icon%20Text))
  (LocalVariables|SetTexture%20Badge Texture)
  (Variables|Default|SetTarget Target)
  (if (Utilities|Array|ContainsItem (Variables|Default|GetBadgeInventory) _output_get)
    (return)
    (else
      (Utilities|Array|Add (Variables|Default|GetBadgeInventory) (Variables|Default|GetIcon%20Text))
      (bind _returnvalue (UserInterface|CreateWidget "/Game/A_BP/Widget/W_BadgeSlot.W_BadgeSlot_C" (Game|GetPlayerController 0) (Variables|Default|GetIcon%20Text) (LocalVariables|GetTexture%20Badge)))
      (Variables|Default|SetTotalBadge (Utilities|Array|Length (Class|PanelWidget|GetAllChildren (Variables|Default|GetTarget))))
      (if (< (Utilities|Array|Length (Class|PanelWidget|GetAllChildren (Variables|Default|GetTarget))) 4)
        (Class|UniformGridPanel|AddChildtoUniformGrid (Variables|Default|GetTarget) _returnvalue 0 (Variables|Default|GetTotalBadge))
        (else
          (Class|UniformGridPanel|AddChildtoUniformGrid (Variables|Default|GetTarget) _returnvalue 1 (- (Variables|Default|GetTotalBadge) 4))))
      (Audio|PlaySound2D "/Engine/VREditor/Sounds/UI/Click_on_Button.Click_on_Button" 1.0 1.0 0.0 0 0)
      (return))))

(fn NewFunction0)