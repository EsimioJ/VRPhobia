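; A physics-enabled picture frame actor whose image can be switched from the keyboard and that can be picked up and dropped.
; On BeginPlay it enables input and creates a dynamic material from the Picture mesh's material.
; Keys 1 and 2 set its "foto" texture parameter to one of two snake cartoon textures.
; Pickup disables Frame physics and attaches the root to the given component; Drop re-enables physics and detaches.
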(event EventBeginPlay
  (Input|EnableInput (Game|GetPlayerController 0))
  (bind _returnvalue (Rendering|Material|CreateDynamicMaterialInstance (Rendering|Material|GetMaterial (Variables|Default|GetPicture) 0) "foto" "None" :!class /Script/Engine.KismetMaterialLibrary))
  (Variables|Default|SetDyn_Material_instance _returnvalue))

(event EventPickup
  (params (AttachTo :type Scene%20Component%20Object%20Reference))
  (Physics|SetSimulatePhysics (Variables|Default|GetFrame) false)
  (Transformation|AttachComponentToComponent (VehicleSound|GetRootComponent) AttachTo "None" "KeepWorld" "KeepWorld" "KeepWorld" false))

(event EventDrop
  (Physics|SetSimulatePhysics (Variables|Default|GetFrame) true)
  (Transformation|DetachFromActor "KeepWorld" "KeepWorld" "KeepWorld"))

(event Input|KeyboardEvents|1
  (params (Key :type Key%20Structure :default "None"))
  (:Pressed
    (Rendering|Material|SetTextureParameterValue (Variables|Default|GetDyn_Material_instance) "foto" "/Game/A_BP/Pictures/snakecartoon.snakecartoon")
    (Rendering|Material|SetMaterial (Variables|Default|GetPicture) 0 (Variables|Default|GetDyn_Material_instance))))

(event Input|KeyboardEvents|2
  (params (Key :type Key%20Structure :default "None"))
  (:Pressed
    (Utilities|FlowControl|Sequence
      (:then_0
        (Rendering|Material|SetTextureParameterValue (Variables|Default|GetDyn_Material_instance) "foto" "/Game/A_BP/Materials/snakecartoon2.snakecartoon2"))
      (:then_1
        (Rendering|Material|SetMaterial (Variables|Default|GetPicture) 0 (Variables|Default|GetDyn_Material_instance))))))

(fn ConstructionScript)